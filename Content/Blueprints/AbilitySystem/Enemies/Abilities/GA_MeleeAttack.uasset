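; Enemy melee attack gameplay ability that turns the avatar toward its combat target and plays a random attack montage from its combat interface.
; When the montage's tagged gameplay event arrives, it finds live players within a small sphere around that tag's combat socket and damages non-friendly ones.
; The ability ends after the hit check, when the montage completes or is interrupted, or if no montages exist.
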(event `self.K2_ActivateAbility`
  (bind _returnvalue (`self.GetAvatarActorFromActorInfo`))
  (bind _returnvalue_2 (`self.GetAvatarActorFromActorInfo`))
  (bind _returnvalue_3 (message `EnemyInterface.GetCombatTarget` _returnvalue))
  (bind _ascombat_interface (cast `CombatInterface` _returnvalue))
  (`CombatInterface.UpdateFacingTarget` _ascombat_interface (`Actor.K2_GetActorLocation` _returnvalue_3))
  (bind _output (`self.GetRandomMontage`))
  (bind (_montage _montagetag) (break `TaggedMontage` _output))
  (`AbilityTask_PlayMontageAndWait.CreatePlayMontageAndWaitProxy` "None" _montage
    (:`then`
      (`AbilityTask_WaitGameplayEvent.WaitGameplayEvent` _montagetag null
        (:`EventReceived`
          (bind _returnvalue_4 (message `CombatInterface.GetCombatSocketLocation` _returnvalue_2 _montagetag))
          (bind _outoverlappingactors (`AuraAbilitySystemLibrary.GetLivePlayersWithinRadius` _returnvalue_2 (`|MakeArray` _returnvalue_2) 45.0 _returnvalue_4))
          (for _array_element _outoverlappingactors
            (if (`AuraAbilitySystemLibrary.IsNotFriend` (`self.GetAvatarActorFromActorInfo`) _array_element)
              (`self.CauseDamage` _array_element)))
          (`self.K2_EndAbility`))))
    (:`OnCompleted`
      (`self.K2_EndAbility` :!label _label))
    (:`OnInterrupted`
      (goto _label))
    (:`OnCancelled`
      (goto _label))))

(fn `GetRandomMontage`
  (returns (Output :type "TaggedMontage Structure (by ref)"))
  (bind _returnvalue (message `CombatInterface.GetAttackMontages` (`self.GetAvatarActorFromActorInfo`)))
  (bind _returnvalue_2 (`KismetArrayLibrary.Array_Length` _returnvalue))
  (if (> _returnvalue_2 0)
    (return (`|GetArrayItem` _returnvalue (`KismetMathLibrary.RandomIntegerInRange` 0 (- _returnvalue_2 1))))
    (else
      (`self.K2_EndAbility`))))