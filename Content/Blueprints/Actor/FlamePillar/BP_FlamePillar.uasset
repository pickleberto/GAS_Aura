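; BP_FlamePillar is a flame pillar actor that flickers its FlameLight with randomly varying intensity.
; From BeginPlay, ChooseTimeline randomly starts one of four flame intensity timelines, and each one calls it again on finishing to form an endless loop.
; While a timeline runs, ScaleFlameIntensity multiplies its curve value by BaseIntensity and applies the result to the light.
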(event `ChooseTimeline`
  (switch `int` (`KismetMathLibrary.RandomIntegerInRange` 0 3)
    (:`Default`
      (`self.PlayTimeline4` :!label _label))
    (:`0`
      (`self.PlayTimeLine1`))
    (:`1`
      (`self.PlayTimeline2`))
    (:`2`
      (`self.PlayTimeline3`))
    (:`3`
      (goto _label))))

(event `self.ReceiveBeginPlay`
  (`self.ChooseTimeline`))

(event `PlayTimeLine1`
  (bind (_direction _flameintensity) (`Timeline|FlameIntensityTimeline_1` :!via `PlayFromStart`)
    (:`Update`
      (`self.ScaleFlameIntensity` _flameintensity))
    (:`Finished`
      (`self.ChooseTimeline`))))

(event `PlayTimeline2`
  (bind (_direction _flameintensity) (`Timeline|FlameIntensityTimeline_2` :!via `PlayFromStart`)
    (:`Update`
      (`self.ScaleFlameIntensity` _flameintensity))
    (:`Finished`
      (`self.ChooseTimeline`))))

(event `PlayTimeline3`
  (bind (_direction _flameintensity) (`Timeline|Timeline_3` :!via `PlayFromStart`)
    (:`Update`
      (`self.ScaleFlameIntensity` _flameintensity))
    (:`Finished`
      (`self.ChooseTimeline`))))

(event `PlayTimeline4`
  (bind (_direction _flameintensity) (`Timeline|Timeline_4` :!via `PlayFromStart`)
    (:`Update`
      (`self.ScaleFlameIntensity` _flameintensity))
    (:`Finished`
      (`self.ChooseTimeline`))))

(fn `ScaleFlameIntensity`
  (params (A :type "Float (double-precision)"))
  (`LightComponent.SetIntensity` (`self.FlameLight`) (* A (`self.BaseIntensity`))))

(fn `UserConstructionScript`)