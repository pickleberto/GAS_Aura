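; BP_Checkpoint is a checkpoint actor that plays a glow and spinning magic circle effect when reached.
; On CheckpointReached, a timeline drives the Glow parameter of the passed-in dynamic material instance, scaled by GlowFactor, and rolls the circle decal by SpinFactor each update.
; HighlightActor and UnHighlightActor toggle custom depth rendering on the checkpoint mesh.
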(event `self.CheckpointReached`
  (params (DynamicMaterialInstance :type "MaterialInstanceDynamic Object Reference"))
  (bind (_direction _glowtrack) (`Timeline|GlowTimeline`)
    (:`Update`
      (`MaterialInstanceDynamic.SetScalarParameterValue` DynamicMaterialInstance "Glow" (* _glowtrack (`self.GlowFactor`)))
      (`SceneComponent.K2_AddLocalRotation` (`self.MagicCircleDecal`) (`KismetMathLibrary.MakeRotator` (`self.SpinFactor`)) false false))))

(event `HighlightInterface.HighlightActor`
  (`PrimitiveComponent.SetRenderCustomDepth` (`self.CheckpointMesh`) true))

(event `HighlightInterface.UnHighlightActor`
  (`PrimitiveComponent.SetRenderCustomDepth` (`self.CheckpointMesh`) false))

(fn `UserConstructionScript`)