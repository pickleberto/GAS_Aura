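; Enemy ranged attack gameplay ability that fires a projectile at the avatar's current combat target.
; On activation it snapshots the target's location, turns the avatar toward it through the combat interface, and plays a randomly chosen attack montage.
; The montage's gameplay event tag triggers the projectile spawn from that montage's socket, with optional pitch override.
; The ability ends when the montage completes, is interrupted or cancelled, or none are available.
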(event `self.K2_ActivateAbility`
  (bind _returnvalue (`self.GetAvatarActorFromActorInfo`))
  (bind _returnvalue_2 (message `EnemyInterface.GetCombatTarget` _returnvalue))
  (set `self.TargetLocation` (`Actor.K2_GetActorLocation` _returnvalue_2))
  (bind _ascombat_interface (cast `CombatInterface` _returnvalue))
  (`CombatInterface.UpdateFacingTarget` _ascombat_interface (`self.TargetLocation`))
  (bind _output (`self.GetRandomMontage_abe`))
  (bind (_montage _montagetag _sockettag) (break `TaggedMontage` _output))
  (`AbilityTask_PlayMontageAndWait.CreatePlayMontageAndWaitProxy` "None" _montage 1.0 "None" false
    (:`then`
      (`AbilityTask_WaitGameplayEvent.WaitGameplayEvent` _montagetag null true
        (:`EventReceived`
          (`self.SpawnProjectile` (`self.TargetLocation`) _sockettag (`self.ShouldOverridePitch`) (`self.PitchOverride`)))))
    (:`OnCompleted`
      (`self.K2_EndAbility` :!label _label))
    (:`OnInterrupted`
      (goto _label))
    (:`OnCancelled`
      (goto _label))))

(fn `GetRandomMontage_abe`
  (returns (Output :type "TaggedMontage Structure"))
  (bind _returnvalue (message `CombatInterface.GetAttackMontages` (`self.GetAvatarActorFromActorInfo`)))
  (bind _returnvalue_2 (`KismetArrayLibrary.Array_Length` _returnvalue))
  (if (> _returnvalue_2 0)
    (return (`|GetArrayItem` _returnvalue (`KismetMathLibrary.RandomIntegerInRange` 0 (- _returnvalue_2 1))))
    (else
      (`self.K2_EndAbility`))))